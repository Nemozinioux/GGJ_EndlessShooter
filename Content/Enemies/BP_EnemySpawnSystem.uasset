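; Wave spawner that sends growing waves of BP_BaseEnemy at the player from four random spawn points.
; Each wave opens with a burst sized by WaveNumber, then trickles in enemies at a faster rate each wave, setting walk speed through each enemy's SpeedEnemiesUp.
; After the trickle, it increments the wave and raises the next count.
; Enemy deaths empty SpawnedEnemies, and a delayed recheck triggers the player's WaveFinished and upgrade widget update.
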(event `self.ReceiveBeginPlay`
  (bind _asbp_first_person_character (cast `/Game/FirstPerson/Blueprints/BP_FirstPersonCharacter` (`GameplayStatics.GetPlayerCharacter` 0)))
  (bind _output_get (set `self.PlayerCharacter` _asbp_first_person_character))
  (set `/Game/FirstPerson/Blueprints/BP_FirstPersonCharacter.Spawner` self _output_get)
  (`self.BeginNewWave`))

(event `BeginNewWave`
  (bind _index (`self.Index`))
  ;[1 1 1] Spawns a first blob of enemies to start waves progressively harder
  (`KismetSystemLibrary.Delay` 3.0)
  (`KismetSystemLibrary.PrintString` (`KismetStringLibrary.Conv_IntToString` (`self.EnemiesToSpawn`)))
  (`|ExecutionSequence`
    (:`then_0`
      (for _ (range (+ (* (* (`self.WaveNumber`) 2) 2) 1))
        (bind _returnvalue (`|SpawnActorFromClass` "/Game/Enemies/BP_BaseEnemy.BP_BaseEnemy_C" (`SceneComponent.K2_GetComponentToWorld` (`|GetArrayItem` (`self.Spawns`) (`KismetMathLibrary.RandomIntegerInRange` 0 3))) "AdjustIfPossibleButAlwaysSpawn" "MultiplyWithRoot" null null))
        (`/Engine/EditorBlueprintResources/StandardMacros.IsValid` _returnvalue
          (:`Is Valid`
            (set `/Game/Enemies/BP_BaseEnemy.Manager` self _returnvalue)
            (bind (_returnvalue_2 _charactermovement) (`self.SpeedEnemiesUp` _returnvalue))
            (set `CharacterMovementComponent.MaxWalkSpeed` _returnvalue_2 _charactermovement)
            (`KismetArrayLibrary.Array_Add` (`self.SpawnedEnemies`) _returnvalue)))))
    (:`then_1`
      (`KismetSystemLibrary.Delay` 1.0)
      (if (> (`self.EnemiesToSpawn`) 0)
        (bind _returnvalue_3 (`|SpawnActorFromClass` "/Game/Enemies/BP_BaseEnemy.BP_BaseEnemy_C" (`SceneComponent.K2_GetComponentToWorld` (`|GetArrayItem` (`self.Spawns`) (`KismetMathLibrary.RandomIntegerInRange` 0 3))) "AdjustIfPossibleButAlwaysSpawn" "MultiplyWithRoot" null null :!label _label))
        (`/Engine/EditorBlueprintResources/StandardMacros.IsValid` _returnvalue_3
          (:`Is Valid`
            (set `/Game/Enemies/BP_BaseEnemy.Manager` self _returnvalue_3)
            (bind (_returnvalue_4 _charactermovement_2) (`self.SpeedEnemiesUp` _returnvalue_3))
            (set `CharacterMovementComponent.MaxWalkSpeed` _returnvalue_4 _charactermovement_2)
            (`KismetArrayLibrary.Array_Add` (`self.SpawnedEnemies`) _returnvalue_3)
            (`/Engine/EditorBlueprintResources/StandardMacros.IncrementInt` _index
              (:`  `
                (`KismetSystemLibrary.Delay` (/ 1.0 (`KismetMathLibrary.Conv_IntToDouble` (`self.WaveNumber`))))
                (if (>= _index (`self.EnemiesToSpawn`))
                  (`/Engine/EditorBlueprintResources/StandardMacros.IncrementInt` (`self.WaveNumber`)
                    (:`  `
                      (set `self.Index` 0)
                      (set `self.EnemiesToSpawn` (+ (`self.EnemiesToSpawn`) (+ (`KismetMathLibrary.Clamp` (* (- (`self.WaveNumber`) 3) 10) 0 10000000) (* (`self.WaveNumber`) 5))))))
                  (else
                    (goto _label)))))))
        (else
          (set `self.Index` 0))))))

(event `EnemyDied`
  (params (Source :type "/Game/Enemies/BP_BaseEnemy Object Reference"))
  (bind _spawnedenemies (`self.SpawnedEnemies`))
  (`/Engine/EditorBlueprintResources/StandardMacros.IsValid` Source
    (:`Is Valid`
      (`KismetArrayLibrary.Array_RemoveItem` _spawnedenemies Source)
      (if (`KismetArrayLibrary.Array_IsEmpty` _spawnedenemies)
        (`self.LevelEndTimer`)))))

(event `LevelEndTimer`
  (`KismetSystemLibrary.Delay` 2.0)
  (if (`KismetArrayLibrary.Array_IsEmpty` (`self.SpawnedEnemies`))
    (`/Game/FirstPerson/Blueprints/BP_FirstPersonCharacter.WaveFinished` (`self.PlayerCharacter`))
    (`/Game/Widgets/WB_Upgrades.UpdateWave` (`/Game/FirstPerson/Blueprints/BP_FirstPersonCharacter.UpgradeWidget` (`self.PlayerCharacter`)) (`self.WaveNumber`))))

(fn `UserConstructionScript`
  (bind _spawns (`self.Spawns`))
  (`KismetArrayLibrary.Array_Add` _spawns (`self.Spawn1`))
  (`KismetArrayLibrary.Array_Add` _spawns (`self.Spawn2`))
  (`KismetArrayLibrary.Array_Add` _spawns (`self.Spawn3`))
  (`KismetArrayLibrary.Array_Add` _spawns (`self.Spawn4`)))