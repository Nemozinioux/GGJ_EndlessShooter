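; Base enemy pawn that chases the player and can be killed for points.
; From BeginPlay it runs AIMoveTo toward the player, re-issuing the move after a short delay on either success or failure.
; Its TakeDamage event subtracts Health and, at zero or below, notifies its Manager of the death, awards points to the BP_FirstPersonCharacter player and destroys the enemy.
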(event `self.ReceiveBeginPlay`
  (`self.WalkUpToPlayer`))

(event `TakeDamage`
  (params (Damage :type Integer))
  (bind _output_get (set `self.Health` (- (`self.Health`) Damage)))
  (if (<= _output_get 0)
    (`/Game/Enemies/BP_EnemySpawnSystem.EnemyDied` (`self.Manager`) self)
    (bind _asbp_first_person_character (cast `/Game/FirstPerson/Blueprints/BP_FirstPersonCharacter` (`GameplayStatics.GetPlayerCharacter` 0)))
    (`/Game/FirstPerson/Blueprints/BP_FirstPersonCharacter.GainPoints` _asbp_first_person_character 100)
    (`self.K2_DestroyActor`)))

(event `WalkUpToPlayer`
  (`|AIMoveTo` self (0.0 0.0 0.0) (`GameplayStatics.GetPlayerCharacter` 0)
    (:`OnSuccess`
      _)
    (:`OnFail`
      _))
  (`KismetSystemLibrary.Delay` 0.2)
  (`self.WalkUpToPlayer`))

(fn `UserConstructionScript`)